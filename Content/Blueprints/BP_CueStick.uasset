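; BP_CueStick is a two-handed VR cue stick that gives haptic feedback and scores on hits.
; Each Tick, a held back grip moves the stick to the back handle, and a held front grip aims it from back to front handle.
; An unheld front handle reattaches to the root.
; Any overlap on the End component triggers the VRPawn's ball-hit haptic and increments the score in Menu2's widget.
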(event `self.ReceiveTick`
  (params (DeltaSeconds :type "Float (single-precision)"))
  (if (`/Game/VRTemplate/Blueprints/GrabComponent.bIsHeld` (`self.FrontGrabComponent`))
    (`self.K2_SetActorRotation` (`KismetMathLibrary.FindLookAtRotation` (`SceneComponent.K2_GetComponentLocation` (`self.HandleBack`)) (`SceneComponent.K2_GetComponentLocation` (`self.HandleFront`))))
    (else
      (`SceneComponent.K2_AttachToComponent` (`self.HandleFront`) (`self.CueStickRoot`) "None" "KeepWorld" "KeepWorld" "KeepWorld" true)))
  (if (`/Game/VRTemplate/Blueprints/GrabComponent.bIsHeld` (`self.BackGrabComponent`))
    (`self.K2_SetActorLocation` (`SceneComponent.K2_GetComponentLocation` (`self.HandleBack`)))))

(event `self.End.OnComponentBeginOverlap`
  (params (OverlappedComponent :type "PrimitiveComponent Object Reference") (OtherActor :type "Actor Object Reference") (OtherComp :type "PrimitiveComponent Object Reference") (OtherBodyIndex :type Integer) (bFromSweep :type Boolean) (SweepResult :type "HitResult Structure (by ref)"))
  (bind _returnvalue (`GameplayStatics.GetActorOfClass` "/Game/VRTemplate/Blueprints/VRPawn.VRPawn_C"))
  (`/Game/VRTemplate/Blueprints/VRPawn.TriggerBallHitHaptic` _returnvalue)
  (bind _returnvalue_2 (`GameplayStatics.GetActorOfClass` "/Game/UI/Menu2.Menu2_C"))
  (bind _asmenu_2 (cast `/Game/UI/Menu2` _returnvalue_2))
  (bind _aswidget_menu_2 (cast `/Game/UI/WidgetMenu2` (`WidgetComponent.GetWidget` (`/Game/UI/Menu2.Widget` _asmenu_2))))
  (`/Game/UI/WidgetMenu2.IncrementScore` _aswidget_menu_2))

(fn `UserConstructionScript`)