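; BP_Ball is a physics ball that gets pulled into a BP_Hole when it overlaps one while in game.
; On overlap it saves its velocity, ignores a custom collision channel, disables physics and uses a Timeline to lerp to the hole's location.
; When the Timeline finishes, it restores physics, enables gravity and applies a small impulse along the saved direction.
; Ending the hole overlap clears InGame.
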(event `self.ReceiveActorBeginOverlap`
  (params (OtherActor :type "Actor Object Reference"))
  (bind _sphere (`self.Sphere`))
  (bind _sphere_2 (`self.Sphere`))
  (bind _asbp_hole (cast `/Game/Blueprints/BP_Hole` OtherActor))
  (if (`self.InGame`)
    (set `self.TargetLocation` (`SceneComponent.K2_GetComponentLocation` (`Actor.RootComponent` _asbp_hole)))
    (set `self.StartLocatrion` (`SceneComponent.K2_GetComponentLocation` (`self.Sphere`)))
    (set `self.Velocity` (`self.GetVelocity`))
    (`PrimitiveComponent.SetCollisionResponseToChannel` _sphere "ECC_GameTraceChannel4" "ECR_Ignore")
    (`PrimitiveComponent.SetSimulatePhysics` _sphere false)
    (bind (_direction _newtrack_0) (`Timeline|Timeline` :!via `PlayFromStart`)
      (:`Update`
        (`SceneComponent.K2_SetWorldLocation` (`self.Sphere`) (`KismetMathLibrary.VLerp` (`self.StartLocatrion`) (`self.TargetLocation`) _newtrack_0) false false))
      (:`Finished`
        (`PrimitiveComponent.SetSimulatePhysics` _sphere_2 true)
        (`PrimitiveComponent.SetEnableGravity` _sphere_2 true)
        (`PrimitiveComponent.AddImpulse` _sphere_2 (* (`KismetMathLibrary.Normal` (`self.Velocity`)) 25) "None" false)))))

(event `self.ReceiveActorEndOverlap`
  (params (OtherActor :type "Actor Object Reference"))
  (cast `/Game/Blueprints/BP_Hole` OtherActor)
  (set `self.InGame` false))

(fn `UserConstructionScript`)