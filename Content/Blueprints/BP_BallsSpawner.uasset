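; Billiards ball spawner actor that builds a pyramid of BP_Ball actors plus a cue ball.
; BuildBallsPyramid places each ball from a per-index offset map, while ball 0 gets a random integer-shifted position around Box1.
; Each ball receives a mesh and mapped material, the cue ball a mass override, then attaches to an externally supplied container.
; BeginPlay is empty, and its own graph leaves the build and container-transform calls unwired.
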(event `self.ReceiveBeginPlay`)

(fn `BuildBallsPyramid`
  (for _index (range 15)
    (if (== _index 0)
      (`self.SetBallPositionCue`)
      (else
        (`self.SetBallPositionPyramid` _index)))
    (bind _returnvalue (`|SpawnActorFromClass` "/Game/Blueprints/BP_Ball.BP_Ball_C" (`KismetMathLibrary.MakeTransform` (`self.BallPosition`)) "Undefined" "MultiplyWithRoot" null null))
    (`self.SetBallProperties` _returnvalue _index)))

(fn `GenerateCoordinateShiftFromExtent`
  (params (Extent :type "Vector Structure"))
  (returns (Shift :type "Vector Structure"))
  (bind _returnvalue (`KismetMathLibrary.FTrunc` Extent_X))
  (bind _returnvalue_2 (`KismetMathLibrary.FTrunc` Extent_Y))
  (bind _returnvalue_3 (`KismetMathLibrary.FTrunc` Extent_Z))
  (bind _result (`/Engine/EditorBlueprintResources/StandardMacros.NegateInt` _returnvalue)
    (:`  `
      (bind _result_2 (`/Engine/EditorBlueprintResources/StandardMacros.NegateInt` _returnvalue_2)
        (:`  `
          (bind _result_3 (`/Engine/EditorBlueprintResources/StandardMacros.NegateInt` _returnvalue_3)
            (:`  `
              (return (`KismetMathLibrary.MakeVector` (`KismetMathLibrary.Conv_IntToDouble` (`KismetMathLibrary.RandomIntegerInRange` _result _returnvalue)) (`KismetMathLibrary.Conv_IntToDouble` (`KismetMathLibrary.RandomIntegerInRange` _result_2 _returnvalue_2)) (`KismetMathLibrary.Conv_IntToDouble` (`KismetMathLibrary.RandomIntegerInRange` _result_3 _returnvalue_3)))))))))))

(fn `SetBallPositionCue`
  (bind _box1 (`self.Box1`))
  (bind _shift (`self.GenerateCoordinateShiftFromExtent` (`BoxComponent.GetScaledBoxExtent` _box1)))
  (set `self.BallPosition` (+ _shift (`SceneComponent.K2_GetComponentLocation` _box1))))

(fn `SetBallPositionPyramid`
  (params (BallIndex :type "Integer (by ref)"))
  (bind _returnvalue_location (`KismetMathLibrary.BreakTransform` (`self.GetTransform`)))
  (set `self.BallPosition` (+ _returnvalue_location (`BlueprintMapLibrary.Map_Find` (`self.BalltoShiftMap`) BallIndex))))

(fn `SetBallProperties`
  (params (Ball :type "/Game/Blueprints/BP_Ball Object Reference") (BallIndex :type "Integer (by ref)"))
  (bind _sphere (`/Game/Blueprints/BP_Ball.Sphere` Ball))
  (`StaticMeshComponent.SetStaticMesh` _sphere "/Engine/EngineMeshes/Sphere.Sphere")
  (`PrimitiveComponent.SetMaterial` _sphere 0 (`BlueprintMapLibrary.Map_Find` (`self.BalltoMatMap`) BallIndex))
  (if (== BallIndex 0)
    (`PrimitiveComponent.SetMassOverrideInKg` _sphere "None" 0.25 true))
  (`self.K2_AttachToActor` (`local.Ball`) (`self.BallsContainer`) "None" "KeepWorld" "KeepWorld" "KeepWorld" true))

(fn `SetBallsContainerTransform`
  (`self.K2_SetActorTransform` (`self.BallsContainer`) (`SceneComponent.K2_GetComponentToWorld` (`self.Box`)) false false))

(fn `UpdateBallsContainer`
  (params (Container :type "Actor Object Reference"))
  (set `self.BallsContainer` Container))

(fn `UserConstructionScript`)